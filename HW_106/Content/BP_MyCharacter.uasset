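; Player character for a coin-collecting platformer, handling movement, pickups, respawning and the transition to Level2.
; Movement follows control rotation, and jumping requires a downward line trace from the Cube component to hit a Ground-tagged actor.
; Hitting coins destroys them and decrements CoinsLeft; overlapping a Trigger-tagged actor opens Level2 only when that count equals 4.
; Tick updates walk speed and teleports the player to Respawn below KillZone height.
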(event `self.ReceiveActorBeginOverlap`
  (params (OtherActor :type "Actor Object Reference"))
  ;[1 1 1] OpenLevel
  (if (`self.ActorHasTag` OtherActor "Trigger")
    (if (== (`self.Coins Left`) 4)
      (`GameplayStatics.OpenLevel` "Level2"))))

(event `self.ReceiveHit`
  (params (MyComp :type "PrimitiveComponent Object Reference") (Other :type "Actor Object Reference") (OtherComp :type "PrimitiveComponent Object Reference") (bSelfMoved :type Boolean) (HitLocation :type "Vector Structure") (HitNormal :type "Vector Structure") (NormalImpulse :type "Vector Structure") (Hit :type "HitResult Structure (by ref)"))
  (bind (_bblockinghit _binitialoverlap _time _distance _location _impactpoint _normal _impactnormal _physmat _hitactor) (`GameplayStatics.BreakHitResult` Hit))
  ;[1 1 1] DestroyCoin
  (if (`self.ActorHasTag` _hitactor "Coin")
    (bind _ascoin (cast `/Game/Coin` _hitactor))
    (`self.K2_DestroyActor` _ascoin)
    (`KismetSystemLibrary.PrintString` "Collected a coin!")
    (set `self.Coins Left` (- (`self.Coins Left`) 1))))

(event `InputAction|Jump`
  (params (Key :type "Key Structure"))
  (bind _returnvalue (`SceneComponent.K2_GetComponentLocation` (`self.Cube`)))
  ;[1 1 1] Jump/LineTrace
  (:`Pressed`
    (bind _outhit (`KismetSystemLibrary.LineTraceSingle` _returnvalue (+ _returnvalue (* (0.0 0.0 -1.0) (`self.Distance`))) "TraceTypeQuery1"))
    (if (`self.ActorHasTag` (`.HitActor` (`GameplayStatics.BreakHitResult` _outhit)) "Ground")
      (`KismetSystemLibrary.PrintString` "Jumping on Ground")
      (`self.Jump`)
      (else
        (`KismetSystemLibrary.PrintString` "Not on Ground")))))

(event `InputAxis|MoveForward`
  (params (AxisValue :type "Float (single-precision)"))
  ;[1 1 1] MoveForward/Backward
  (`self.AddMovementInput` (`KismetMathLibrary.GetForwardVector` (`self.GetControlRotation`)) AxisValue))

(event `InputAxis|MoveRight`
  (params (AxisValue :type "Float (single-precision)"))
  ;[1 1 1] MoveRight/Left
  (`self.AddMovementInput` (`KismetMathLibrary.GetRightVector` (`self.GetControlRotation`)) AxisValue))

(event `self.ReceiveTick`
  (params (DeltaSeconds :type "Float (single-precision)"))
  ;[1 1 1] MovementSpeed/Respawn
  (set `CharacterMovementComponent.MaxWalkSpeed` (* (`self.SpeedMultiplier`) (`self.Player Speed`)) (`self.CharacterMovement`))
  (if (< (.z (`SceneComponent.K2_GetComponentLocation` (`self.Cube`))) (`self.KillZone`))
    (`self.K2_TeleportTo` (`self.Respawn`))
    (`KismetSystemLibrary.PrintString` "Respawned")))

(fn `UserConstructionScript`)